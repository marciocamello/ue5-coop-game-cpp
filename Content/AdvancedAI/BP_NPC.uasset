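; BP_NPC is an AI-controlled NPC Blueprint that runs a behavior tree and shows debug feedback when damaged.
; On BeginPlay its AI controller starts the BT_NPC behavior tree.
; Point damage draws a brief debug sphere and the damage amount at the hit location.
; Its HealthComp's health-change event prints the current health in red at the actor's location.
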(event OnHealthChanged(HealthComp)
  (params (HealthComp :type S%20Health%20Component%20Object%20Reference) (Health :type Float%20%28single-precision%29) (HealthDelta :type Float%20%28single-precision%29) (DamageType :type Damage%20Type%20Object%20Reference) (InstigatedBy :type Controller%20Object%20Reference) (DamageCauser :type Actor%20Object%20Reference))
  (Rendering|Debug|DrawDebugString (Transformation|GetActorLocation) (Utilities|String|ToString(Float) Health) 0 "(R=1.000000,G=0.000000,B=0.000000,A=1.000000)" 1.0))

(event EventBeginPlay
  (AI|RunBehaviorTree (AI|GetAIController self) "/Game/AdvancedAI/BT_NPC.BT_NPC"))

(event Game|Damage|EventPointDamage
  (params (Damage :type Float%20%28single-precision%29) (DamageType :type Damage%20Type%20Object%20Reference) (HitLocation :type Vector :default "0, 0, 0") (HitNormal :type Vector :default "0, 0, 0") (HitComponent :type Primitive%20Component%20Object%20Reference) (BoneName :type Name :default "None") (ShotFromDirection :type Vector :default "0, 0, 0") (InstigatedBy :type Controller%20Object%20Reference) (DamageCauser :type Actor%20Object%20Reference) (HitInfo :type Hit%20Result%20Structure%20%28by%20ref%29))
  (Rendering|Debug|DrawDebugSphere HitLocation 5.0 12 "(R=0.973958,G=0.475949,B=0.000000,A=1.000000)" 1.0 1.0)
  (Rendering|Debug|DrawDebugString HitLocation (Utilities|String|ToString(Float) Damage) 0 "(R=1.000000,G=1.000000,B=1.000000,A=1.000000)" 1.0))

(fn ConstructionScript)