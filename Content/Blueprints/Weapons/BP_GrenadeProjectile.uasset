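; Grenade projectile actor that explodes on a fixed one-second fuse started at BeginPlay.
; When the delay ends, the Explode event spawns an explosion particle effect, then radial damage is applied around the actor using its radius and damage type, credited to the instigator's controller.
; The actor then destroys itself and draws a brief debug sphere showing the damage radius.
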(event Custom|Explode
  (Effects|SpawnEmitteratLocation "/Game/WeaponEffects/Explosion/P_Explosion.P_Explosion" (Transformation|GetActorLocation)))

(event EventBeginPlay
  (bind _returnvalue (Transformation|GetActorLocation))
  (Utilities|FlowControl|Delay 1.0)
  (CallFunction|Explode)
  (Game|Damage|ApplyRadialDamage 1e+02 _returnvalue (Variables|Default|GetDamage%20Radius) "/Script/Engine.DamageType" 0 self (Game|GetInstigatorController) false "ECC_Visibility")
  (Actor|DestroyActor)
  (Rendering|Debug|DrawDebugSphere _returnvalue (Variables|Default|GetDamage%20Radius) 12 "(R=1.000000,G=0.865640,B=0.000000,A=1.000000)" 1.0 1.0))

(fn ConstructionScript)