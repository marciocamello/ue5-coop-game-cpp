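; Grenade launcher projectile that explodes on a short fixed timer started at BeginPlay.
; The Explode event spawns the explosion particle and sound, then BeginPlay applies full, non-falloff radial damage within DamageRadius, using a custom trace channel for blocking.
; The actor then destroys itself, with a debug sphere of the damage radius drawn after the destroy call.
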(event Custom|Explode
  (bind _returnvalue (Transformation|GetActorLocation))
  (Effects|SpawnEmitteratLocation "/Game/FX/WeaponEffects/Explosion/P_Explosion.P_Explosion" _returnvalue)
  (Audio|PlaySoundatLocation "/Game/StarterContent/Audio/Explosion01.Explosion01" _returnvalue "0, 0, 0" 1.0 1.0 0.0 0 0 0 0))

(event EventBeginPlay
  (bind _returnvalue (Transformation|GetActorLocation))
  (Utilities|FlowControl|Delay 1.0)
  (CallFunction|Explode)
  (Game|Damage|ApplyRadialDamage 1e+02 _returnvalue (Variables|Default|GetDamage%20Radius) "/Game/Blueprints/Weapons/GrenadeLauncher/DT_GrenadeLaunch.DT_GrenadeLaunch_C" 0 0 0 true "ECC_GameTraceChannel1")
  (Actor|DestroyActor)
  (Rendering|Debug|DrawDebugSphere _returnvalue (Variables|Default|GetDamage%20Radius) 12 "(R=1.000000,G=0.865640,B=0.000000,A=1.000000)" 1.0 1.0))

(fn ConstructionScript)