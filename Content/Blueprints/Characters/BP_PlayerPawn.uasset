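; BP_PlayerPawn is the player pawn Blueprint, handling HUD setup and weapon switching.
; On BeginPlay, only the locally controlled pawn creates crosshair and health indicator widgets and adds them to the viewport.
; Primary and secondary weapon inputs call SpawnWeapon with the rifle or grenade launcher class.
; A disconnected debug print of HealthComp health remains in the graph but never runs.
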(event EventBeginPlay
  (if (Pawn|IsLocallyControlled)
    (Utilities|FlowControl|Sequence
      (:then_0
        ;[1 1 1] Create a crosshair
        (bind _returnvalue (UserInterface|CreateWidget "/Game/UI/W_Crosshair.W_Crosshair_C"))
        (UserInterface|Viewport|AddtoViewport _returnvalue 0))
      (:then_1
        ;[1 1 1] Create a health indicator
        (bind _returnvalue_2 (UserInterface|CreateWidget "/Game/UI/W_HealthIndicator.W_HealthIndicator_C"))
        (UserInterface|Viewport|AddtoViewport _returnvalue_2 0)))))

(event EventTick
  (params (DeltaSeconds :type Float%20%28single-precision%29)))

(event Input|ActionEvents|InputActionPrimaryWeapon
  (params (Key :type Key%20Structure :default "None"))
  ;[1 1 1] Change into Primary/Secondary weapons
  (:Pressed
    (Class|SCharacter|SpawnWeapon "/Game/Blueprints/Weapons/Rifle/BP_Rifle.BP_Rifle_C")))

(event Input|ActionEvents|InputActionSecondaryWeapon
  (params (Key :type Key%20Structure :default "None"))
  ;[1 1 1] Change into Primary/Secondary weapons
  (:Pressed
    (Class|SCharacter|SpawnWeapon "/Game/Blueprints/Weapons/GrenadeLauncher/BP_GrenadeLauncher.BP_GrenadeLauncher_C")))

(fn ConstructionScript)